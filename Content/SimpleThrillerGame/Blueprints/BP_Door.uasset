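; BP_Door is a door Blueprint for a thriller game that swings open and closed and plays random knocking sounds.
; OpenClose uses a FlipFlop to play or reverse a timeline that lerps the root rotation through 90 degrees of yaw, opening slower than it closes, with matching sounds.
; A timer re-arms itself with a new random delay after each knock, played as attenuated audio at the door's location.
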(event Custom|OpenClose
  (bind _defaultsceneroot (Variables|Default|GetDefaultSceneRoot))
  (bind _sound_localization (Variables|Default|GetSound%20Localization))
  (bind _door (Variables|Default|GetDoor))
  (bind _returnvalue (Transformation|GetWorldLocation _door))
  (bind _returnvalue_2 (Transformation|GetWorldRotation _defaultsceneroot))
  (bind (_roll _pitch _yaw) (Math|Rotator|BreakRotator _returnvalue_2))
  ;[0.05098 0.05098 0.05098] Door Animation
  (Utilities|FlowControl|FlipFlop
    (:A
      (Variables|Default|SetBaseRotation _returnvalue_2)
      (Variables|Default|SetTargetRotation (Math|Rotator|MakeRotator _roll _pitch (+ _yaw 9e+01)))
      (Components|Timeline|SetPlayRate (Variables|Default|GetDoorTimeline) 0.3)
      (Audio|PlaySoundatLocation "/Game/SimpleThrillerGame/Sounds/DoorSounds/doorOpen.doorOpen" _returnvalue "0, 0, 0" 1.0 1.0 0.0 _sound_localization 0 0 0)
      (bind _doortrack (Timeline|DoorTimeline Play)
        (:Update
          (Transformation|SetWorldRotation (Variables|Default|GetDefaultSceneRoot) (Math|Rotator|Lerp(Rotator) (Variables|Default|GetBaseRotation) (Variables|Default|GetTargetRotation) _doortrack) false false))))
    (:B
      (Components|Timeline|SetPlayRate (Variables|Default|GetDoorTimeline) 1.0)
      (Audio|PlaySoundatLocation "/Game/SimpleThrillerGame/Sounds/DoorSounds/doorClose.doorClose" _returnvalue "0, 0, 0" 1.0 1.0 0.0 _sound_localization 0 0 0)
      (Timeline|DoorTimeline Reverse))))

(event Custom|PlayKnockKnock
  ;[0.05098 0.05098 0.05098] Knock Knock Sound
  (Audio|PlaySoundatLocation "/Game/SimpleThrillerGame/Sounds/DoorSounds/Knock_Knock.Knock_Knock" (Transformation|GetWorldLocation (Variables|Default|GetDoor)) "0, 0, 0" 1.0 1.0 0.0 (Variables|Default|GetSound%20Localization) 0 0 0)
  (Utilities|Time|SetTimerbyFunctionName 0 "PlayKnockKnock" (Math|Random|RandomFloatinRange 1e+01 1e+02) true true))

(event EventBeginPlay
  ;[0.05098 0.05098 0.05098] Knock Knock Sound
  (Utilities|Time|SetTimerbyFunctionName 0 "PlayKnockKnock" (Math|Random|RandomFloatinRange 1e+01 1e+02) true true))

(fn ConstructionScript)